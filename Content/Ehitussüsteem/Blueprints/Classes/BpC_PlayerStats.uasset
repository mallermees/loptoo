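; BpC_PlayerStats manages the player's stats and shows them on bars in the main widget.
; Initialization stores the player reference and runs stat setup, after which each entry in the stats map initializes its bar with its stat value.
; Stat updates push the current value to the matching bar.
; GetBarForStat maps stat types to widgets, with only Health linked to a bar, the Healthbar.
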(event `InitializeManager`
  (params (Player :type "/Game/FirstPersonBP/Blueprints/FirstPersonCharacter Object Reference"))
  (set `self.PlayerRef` Player)
  (`self.SetUpStats`))

(event `self.OnStatsSetUp`
  (bind _keys (`BlueprintMapLibrary.Map_Keys` (`self.Stats`)))
  (for _array_element _keys
    (`/Game/Ehitussüsteem/Widgets/w_statbar.InitailizeBar` (`self.GetBarForStat` _array_element) (`.StatValue` (`self.GetStat` _array_element)))))

(event `self.UpdateStat`
  (params (Stat :type "/Game/Ehitussüsteem/Blueprints/Enums/e_Stats Enum" :default "NewEnumerator0"))
  (`/Game/Ehitussüsteem/Widgets/w_statbar.UpdateStat` (`self.GetBarForStat` Stat) (`self.GetStat` Stat)))

(fn `GetBarForStat`
  (params (Stat :type "/Game/Ehitussüsteem/Blueprints/Enums/e_Stats Enum" :default "NewEnumerator0"))
  (returns (Bar :type "/Game/Ehitussüsteem/Widgets/w_statbar Object Reference"))
  (return (select `/Game/Ehitussüsteem/Blueprints/Enums/e_Stats` Stat :`NewEnumerator1` (`/Game/Ehitussüsteem/Widgets/W_main.Healthbar` (`/Game/FirstPersonBP/Blueprints/FirstPersonCharacter.MainWidget` (`self.PlayerRef`))))))
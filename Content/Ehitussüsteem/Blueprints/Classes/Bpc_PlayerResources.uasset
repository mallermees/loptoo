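; Player component that manages the building system's resources, their HUD widgets and which resource is currently selected.
; On initialization it has the main widget generate one widget per key of the Resources map, fills in the amounts and highlights the current selection.
; Selection cycles through the map's keys with wraparound, updating the main widget and notifying the building manager.
; Amount changes to the selected resource also notify both, but only in one player state.
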(event `OnResourceSwitched`
  (`/Game/Ehitussüsteem/Blueprints/Classes/Bpc_BuildingManager.OnResourceChanged` (`/Game/FirstPersonBP/Blueprints/FirstPersonCharacter.Bpc_BuildingManager` (`self.PlayerCharacter`))))

(event `InitializeManager`
  (params (Player :type "/Game/FirstPersonBP/Blueprints/FirstPersonCharacter Object Reference"))
  (`/Engine/EditorBlueprintResources/StandardMacros.IsValid` Player
    (:`Is Valid`
      (set `self.PlayerCharacter` Player)
      (set `self.Initialized?` true)
      (bind _createdwidgets (`/Game/Ehitussüsteem/Widgets/W_main.GenerateResourceWidgets` (`/Game/FirstPersonBP/Blueprints/FirstPersonCharacter.MainWidget` (`self.PlayerCharacter`)) self))
      (set `self.ResourceWidgets` _createdwidgets)
      (bind _keys (`BlueprintMapLibrary.Map_Keys` (`self.Resources`)))
      (for _array_element _keys
        (`self.UpdateResourceDisplay` _array_element))
      (`self.SelectCurrentResource`))))

(event `self.UpdateResourceDisplay`
  (params (Resource :type "/Game/Ehitussüsteem/Blueprints/Classes/Bp_master_resource Class Reference"))
  (bind (_success_ _widget) (`self.GetWidgetForResource` Resource))
  (if (`self.Initialized?`)
    (if _success_
      (`TextBlock.SetText` (`/Game/Ehitussüsteem/Widgets/W_Resource.Amount` _widget) (`KismetTextLibrary.Conv_IntToText` (`self.GetResource` Resource) false false))
      (if (and (== (`self.GetSelectedResource`) Resource) (`|EnumEquality` (`/Game/FirstPersonBP/Blueprints/FirstPersonCharacter.State` (`self.PlayerCharacter`)) "NewEnumerator1"))
        (`/Game/Ehitussüsteem/Widgets/W_main.UpdateCurrentResource` (`/Game/FirstPersonBP/Blueprints/FirstPersonCharacter.MainWidget` (`self.PlayerCharacter`)) self)
        (`/Game/Ehitussüsteem/Blueprints/Classes/Bpc_BuildingManager.OnResourceValueModified` (`/Game/FirstPersonBP/Blueprints/FirstPersonCharacter.Bpc_BuildingManager` (`self.PlayerCharacter`)) Resource)))))

(fn `CurrentlySelectedWidget`
  (returns (Widget :type "/Game/Ehitussüsteem/Widgets/W_Resource Object Reference"))
  (return (`.Widget` (`self.GetWidgetForResource` (`self.GetSelectedResource`)))))

(fn `GetSelectedIndex`
  (returns (Out :type Integer))
  (return (`self.SelectedResourceIndex`)))

(fn `GetSelectedResource`
  (returns (Out :type "/Game/Ehitussüsteem/Blueprints/Classes/Bp_master_resource Class Reference"))
  (bind _keys (`BlueprintMapLibrary.Map_Keys` (`self.Resources`)))
  (return (`|GetArrayItem` _keys (`self.SelectedResourceIndex`))))

(fn `GetWidgetForResource`
  (params (Resource :type "/Game/Ehitussüsteem/Blueprints/Classes/Bp_master_resource Class Reference"))
  (returns (`Success?` :type Boolean) (Widget :type "/Game/Ehitussüsteem/Widgets/W_Resource Object Reference"))
  (locals (LocalFound :type "/Game/Ehitussüsteem/Widgets/W_Resource Object Reference"))
  (bind _localfound (`local.LocalFound`))
  (for _array_element (`self.ResourceWidgets`)
    (if (== (`/Game/Ehitussüsteem/Widgets/W_Resource.Resource` _array_element) Resource)
      (set `local.LocalFound` _array_element)
      (break)))
  (`/Engine/EditorBlueprintResources/StandardMacros.IsValid` _localfound
    (:`Is Valid`
      (return true _localfound))
    (:`Is Not Valid`
      (return false null))))

(fn `SelectCurrentResource`
  (`/Game/Ehitussüsteem/Widgets/W_Resource.SelectResource` (`self.CurrentlySelectedWidget`) true false)
  (return))

(fn `SelectNextResource`
  (bind _selectedresourceindex (`self.SelectedResourceIndex`))
  (`/Game/Ehitussüsteem/Widgets/W_Resource.SelectResource` (`self.CurrentlySelectedWidget`) false false)
  (bind _keys (`BlueprintMapLibrary.Map_Keys` (`self.Resources`)))
  (set `self.SelectedResourceIndex` (`KismetMathLibrary.SelectInt` (+ _selectedresourceindex 1) 0 (< _selectedresourceindex (`KismetArrayLibrary.Array_LastIndex` _keys))))
  (`self.SelectCurrentResource`)
  (`/Game/Ehitussüsteem/Widgets/W_main.UpdateCurrentResource` (`/Game/FirstPersonBP/Blueprints/FirstPersonCharacter.MainWidget` (`self.PlayerCharacter`)) self)
  (`self.OnResourceSwitched`))